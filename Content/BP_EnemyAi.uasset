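; Enemy turret-style AI actor that shoots projectiles at the first-person player and can be destroyed by damage.
; On a Tick-driven DoOnce loop it faces the player, waits a random delay, then fires, leading the target by velocity scaled with distance.
; Damage adds to the player's score and updates a widget health bar; death heals the player and destroys the enemy.
; Pawn sensing events are unused.
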(event OnSeePawn(PawnSensing)
  (params (Pawn :type Pawn%20Object%20Reference)))

(event OnHearNoise(PawnSensing)
  (params (Instigator :type Pawn%20Object%20Reference) (Location :type Vector%20%28by%20ref%29 :default "0, 0, 0") (Volume :type Float%20%28single-precision%29)))

(event EventBeginPlay
  (bind _asbp_first_person_character (Utilities|Casting|CastToBP_FirstPersonCharacter (Game|GetPlayerCharacter 0)))
  (Variables|Default|SetPlayerRef _asbp_first_person_character)
  (CallFunction|UpdateHealthBar))

(event Collision|EventActorBeginOverlap
  (params (OtherActor :type Actor%20Object%20Reference)))

(event EventTick
  (params (DeltaSeconds :type Float%20%28single-precision%29))
  (bind _playerref (Variables|Default|GetPlayerRef))
  (bind _firingpoint (Variables|Default|GetFiringPoint))
  (bind _returnvalue (Transformation|GetWorldLocation _firingpoint))
  (bind _capsulecomponent (Variables|/Script/Engine.Character|GetCapsuleComponent _playerref))
  (bind _returnvalue_2 (Transformation|GetWorldLocation _capsulecomponent))
  (Utilities|FlowControl|DoOnce false :!label _label
    (:Completed
      (Transformation|SetActorRotation (Math|Rotator|FindLookatRotation _returnvalue _returnvalue_2))
      (Utilities|FlowControl|Delay (Math|Random|RandomFloatinRange 2.0 6.0))
      (Game|SpawnActorfromClass "/Game/FirstPerson/Blueprints/BP_EnemyProjectile.BP_EnemyProjectile_C" (Math|Transform|MakeTransform _returnvalue (Math|Rotator|FindLookatRotation _returnvalue (+ _returnvalue_2 (* (/ (Transformation|GetDistanceTo _playerref) 5e+03) (Transformation|GetVelocity _playerref))))) "Undefined" 0 0)
      (goto _label Reset))))

(event Game|Damage|EventAnyDamage
  (params (Damage :type Float%20%28single-precision%29) (DamageType :type Damage%20Type%20Object%20Reference) (InstigatedBy :type Controller%20Object%20Reference) (DamageCauser :type Actor%20Object%20Reference))
  (bind _playerref (Variables|Default|GetPlayerRef))
  (bind _playerref_2 (Variables|Default|GetPlayerRef))
  (Variables|/Game/FirstPerson/Blueprints/BP_FirstPersonCharacter.BP_FirstPersonCharacter_C|SetPlayerScore _playerref (+ Damage (Variables|/Game/FirstPerson/Blueprints/BP_FirstPersonCharacter.BP_FirstPersonCharacter_C|GetPlayerScore _playerref)))
  (bind _output_get (Variables|Default|SetHealth (Math|Float|Clamp(Float) (- (Variables|Default|GetHealth) Damage) 0.0 (Variables|Default|GetMaxHealth))))
  (if (== _output_get 0.0)
    (Variables|/Game/FirstPerson/Blueprints/BP_FirstPersonCharacter.BP_FirstPersonCharacter_C|SetHealth _playerref_2 (Math|Float|Clamp(Float) (+ (Variables|/Game/FirstPerson/Blueprints/BP_FirstPersonCharacter.BP_FirstPersonCharacter_C|GetHealth _playerref_2) 1e+02) 0.0 1e+02))
    (Actor|DestroyActor)
    (else
      (CallFunction|UpdateHealthBar))))

(fn ConstructionScript)

(fn UpdateHealthBar
  (bind _asbpw_actor_health_bar (Utilities|Casting|CastToBPW_ActorHealthBar (UserInterface|GetUserWidgetObject (Variables|Default|GetWidget))))
  (Variables|/Game/BPW_ActorHealthBar.BPW_ActorHealthBar_C|SetHealth _asbpw_actor_health_bar (/ (Variables|Default|GetHealth) 1e+02))
  (return))