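; BP_PlayerBoat is the player's boat, which collects wreckage that enters its detection volume and converts it into score.
; On BeginPlay it caches the first-person player character as PlayerRef.
; When WreckageDetect overlaps a BP_Wreckage, it adds a fixed reward to the player's score, cancels the grapple on the player's grapple component, then destroys the wreckage.
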(event OnComponentBeginOverlap(WreckageDetect)
  (params (OverlappedComponent :type Primitive%20Component%20Object%20Reference) (OtherActor :type Actor%20Object%20Reference) (OtherComp :type Primitive%20Component%20Object%20Reference) (OtherBodyIndex :type Integer) (bFromSweep :type Boolean) (SweepResult :type Hit%20Result%20Structure%20%28by%20ref%29))
  (bind _playerref (Variables|Default|GetPlayerRef))
  (bind _asbp_wreckage (Utilities|Casting|CastToBP_Wreckage OtherActor))
  (Variables|/Game/FirstPerson/Blueprints/BP_FirstPersonCharacter.BP_FirstPersonCharacter_C|SetPlayerScore _playerref (+ (Variables|/Game/FirstPerson/Blueprints/BP_FirstPersonCharacter.BP_FirstPersonCharacter_C|GetPlayerScore _playerref) 1e+03))
  (Default|CancelGrapple (Variables|/Game/FirstPerson/Blueprints/BP_FirstPersonCharacter.BP_FirstPersonCharacter_C|GetBP_GrappleComponent _playerref))
  (Actor|DestroyActor _asbp_wreckage))

(event EventBeginPlay
  (bind _asbp_first_person_character (Utilities|Casting|CastToBP_FirstPersonCharacter (Game|GetPlayerCharacter 0)))
  (Variables|Default|SetPlayerRef _asbp_first_person_character))

(event Collision|EventActorBeginOverlap
  (params (OtherActor :type Actor%20Object%20Reference)))

(event EventTick
  (params (DeltaSeconds :type Float%20%28single-precision%29)))

(fn ConstructionScript)