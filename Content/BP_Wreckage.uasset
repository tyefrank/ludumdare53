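; BP_Wreckage is a wreckage actor that drifts on an InterpToMovement component and can be halted while grappled.
; BeginPlay caches the first-person character, randomizes the movement duration and restarts movement, then attempts to cache a grapple hook from the player controller's parent actor.
; When anything begins overlapping WreckageDetect, movement stops if the character's grapple component has this wreckage as its hit actor.
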(event OnComponentBeginOverlap(WreckageDetect)
  (params (OverlappedComponent :type Primitive%20Component%20Object%20Reference) (OtherActor :type Actor%20Object%20Reference) (OtherComp :type Primitive%20Component%20Object%20Reference) (OtherBodyIndex :type Integer) (bFromSweep :type Boolean) (SweepResult :type Hit%20Result%20Structure%20%28by%20ref%29))
  (if (== (Variables|/Game/FirstPerson/Blueprints/BP_GrappleComponent.BP_GrappleComponent_C|GetHitActor (Variables|/Game/FirstPerson/Blueprints/BP_FirstPersonCharacter.BP_FirstPersonCharacter_C|GetBP_GrappleComponent (stale EventBeginPlay _asbp_first_person_character))) self)
    (Components|Movement|StopMovementImmediately (Variables|Default|GetInterpToMovement))))

(event OnComponentEndOverlap(WreckageDetect)
  (params (OverlappedComponent :type Primitive%20Component%20Object%20Reference) (OtherActor :type Actor%20Object%20Reference) (OtherComp :type Primitive%20Component%20Object%20Reference) (OtherBodyIndex :type Integer)))

(event EventBeginPlay
  (bind _interptomovement (Variables|Default|GetInterpToMovement))
  (bind _asbp_first_person_character (Utilities|Casting|CastToBP_FirstPersonCharacter (Game|GetPlayerCharacter 0)))
  (Variables|Default|SetPlayerRef _asbp_first_person_character)
  (bind _output_get (Variables|/Script/Engine.InterpToMovementComponent|SetDuration _interptomovement (Math|Random|RandomFloatinRange 2e+02 4e+02)))
  (Class|InterptoMovementComponent|RestartMovement _interptomovement (/ 1.0 _output_get))
  (bind _asbp_grapple_hook (Utilities|Casting|CastToBP_GrappleHook (Actor|GetParentActor (Game|GetPlayerController 0))))
  (Variables|Default|SetGrappleHookRef _asbp_grapple_hook))

(event Collision|EventActorBeginOverlap
  (params (OtherActor :type Actor%20Object%20Reference)))

(event EventTick
  (params (DeltaSeconds :type Float%20%28single-precision%29)))

(fn ConstructionScript)