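; BP_Pillar is a destructible moving pillar that adds damage taken to the player's score and restores player health when destroyed.
; InterpToMovement moves it over a randomized duration, while a looping timer turns its health bar widget toward the camera.
; Box overlap detaches wreckage and cancels the grapple, or calls ApplyDamage for the player boat with no target set.
; AnyDamage updates the bar or, at zero health, cancels the grapple and destroys the pillar with sound.
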(event OnComponentBeginOverlap(Box)
  (params (OverlappedComponent :type Primitive%20Component%20Object%20Reference) (OtherActor :type Actor%20Object%20Reference) (OtherComp :type Primitive%20Component%20Object%20Reference) (OtherBodyIndex :type Integer) (bFromSweep :type Boolean) (SweepResult :type Hit%20Result%20Structure%20%28by%20ref%29))
  (bind _asbp_wreckage (Utilities|Casting|CastToBP_Wreckage OtherActor)
    (:then
      (Transformation|DetachFromActor _asbp_wreckage "KeepWorld" "KeepWorld" "KeepWorld")
      (Default|CancelGrapple (Variables|/Game/FirstPerson/Blueprints/BP_FirstPersonCharacter.BP_FirstPersonCharacter_C|GetBP_GrappleComponent (Variables|Default|GetPlayerRef))))
    (:CastFailed
      (Utilities|Casting|CastToBP_PlayerBoat OtherActor)
      (Game|Damage|ApplyDamage 0 5e+02 0 0))))

(event Custom|UpdateRotTimer
  (Utilities|Time|SetTimerbyEvent (delegate Custom|UpdateRotation) 0.2 true))

(event Custom|UpdateRotation
  (bind _widget (Variables|Default|GetWidget))
  (Transformation|SetWorldRotation _widget (Math|Rotator|FindLookatRotation (Transformation|GetWorldLocation _widget) (Camera|GetCameraLocation (Game|GetPlayerCameraManager 0))) false false))

(event EventBeginPlay
  (bind _interptomovement (Variables|Default|GetInterpToMovement))
  (bind _asbp_first_person_character (Utilities|Casting|CastToBP_FirstPersonCharacter (Game|GetPlayerCharacter 0)))
  (Variables|Default|SetPlayerRef _asbp_first_person_character)
  (CallFunction|UpdateHealthBar)
  (CallFunction|UpdateRotTimer)
  (bind _output_get (Variables|/Script/Engine.InterpToMovementComponent|SetDuration _interptomovement (Math|Random|RandomFloatinRange 1.5e+02 2e+02)))
  (Class|InterptoMovementComponent|RestartMovement _interptomovement (/ 1.0 _output_get)))

(event Collision|EventActorBeginOverlap
  (params (OtherActor :type Actor%20Object%20Reference)))

(event EventTick
  (params (DeltaSeconds :type Float%20%28single-precision%29)))

(event Game|Damage|EventAnyDamage
  (params (Damage :type Float%20%28single-precision%29) (DamageType :type Damage%20Type%20Object%20Reference) (InstigatedBy :type Controller%20Object%20Reference) (DamageCauser :type Actor%20Object%20Reference))
  (bind _playerref (Variables|Default|GetPlayerRef))
  (bind _playerref_2 (Variables|Default|GetPlayerRef))
  (Variables|/Game/FirstPerson/Blueprints/BP_FirstPersonCharacter.BP_FirstPersonCharacter_C|SetPlayerScore _playerref_2 (+ (Variables|/Game/FirstPerson/Blueprints/BP_FirstPersonCharacter.BP_FirstPersonCharacter_C|GetPlayerScore _playerref_2) Damage))
  (bind _output_get (Variables|Default|SetHealth (Math|Float|Clamp(Float) (- (Variables|Default|GetHealth) Damage) 0.0 (Variables|Default|GetMaxHealth))))
  (if (== _output_get 0.0)
    (Default|CancelGrapple (Variables|/Game/FirstPerson/Blueprints/BP_FirstPersonCharacter.BP_FirstPersonCharacter_C|GetBP_GrappleComponent _playerref))
    (Variables|/Game/FirstPerson/Blueprints/BP_FirstPersonCharacter.BP_FirstPersonCharacter_C|SetHealth _playerref (Math|Float|Clamp(Float) (+ (Variables|/Game/FirstPerson/Blueprints/BP_FirstPersonCharacter.BP_FirstPersonCharacter_C|GetHealth _playerref) 1e+02) 0.0 1e+02))
    (Audio|PlaySoundatLocation "/Game/SoundFX/PillarDestroyed_SFX.PillarDestroyed_SFX" (Transformation|GetActorLocation) "0, 0, 0" 1.0 1.0 0.0 0 0 0 0)
    (Actor|DestroyActor)
    (else
      (CallFunction|UpdateHealthBar))))

(fn ConstructionScript)

(fn UpdateHealthBar
  (bind _asbpw_actor_health_bar (Utilities|Casting|CastToBPW_ActorHealthBar (UserInterface|GetUserWidgetObject (Variables|Default|GetWidget))))
  (Variables|/Game/BPW_ActorHealthBar.BPW_ActorHealthBar_C|SetHealth _asbpw_actor_health_bar (/ (Variables|Default|GetHealth) 2e+02))
  (return))